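; BP_Milk is a milk item actor that serves as the win pickup.
; It binds to its grabbed and dropped events on BeginPlay and records its starting transform.
; When a player-tagged user grabs it, it triggers the player character's win event and opens the win screen level after a short delay.
; When dropped, it teleports back to its starting transform.
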(event Custom|OnItemDropped_Event
  (params (ItemUser :type Pawn%20Object%20Reference))
  (Transformation|SetActorTransform (Variables|Default|GetStartingTransform) false true))

(event Custom|OnItemGrabbed_Event
  (bind _itemuser (Variables|Default|GetItemUser))
  (if (and (Utilities|IsValid _itemuser) (Actor|ActorHasTag _itemuser "Player"))
    (bind _asrg_player_character (Utilities|Casting|CastToRG_PlayerCharacter _itemuser))
    (Default|CallOnPlayerWin _asrg_player_character)
    (Utilities|FlowControl|Delay 5.0)
    (Game|OpenLevel(byObjectReference) "/Game/Levels/L_WinScreen.L_WinScreen")))

(event EventBeginPlay
  (EventDispatchers|AssignOnItemDropped (delegate Custom|OnItemDropped_Event))
  (Variables|Default|SetStartingTransform (Transformation|GetActorTransform))
  (EventDispatchers|AssignOnItemGrabbed (delegate Custom|OnItemGrabbed_Event)))

(event Collision|EventActorBeginOverlap
  (params (OtherActor :type Actor%20Object%20Reference)))

(event EventTick
  (params (DeltaSeconds :type Float%20%28single-precision%29)))

(fn ConstructionScript)