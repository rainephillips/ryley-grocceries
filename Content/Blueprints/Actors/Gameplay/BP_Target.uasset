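; BP_Target is a shootable gameplay target actor that takes damage and is destroyed when its health runs out.
; DealDamage subtracts the incoming damage from Health and calls OnHealthZero at zero or below, which destroys the actor.
; GetHealth exposes the current value, and IsShootable returns true for any interactor.
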(event EventBeginPlay)

(event Collision|EventActorBeginOverlap
  (params (OtherActor :type Actor%20Object%20Reference)))

(event EventTick
  (params (DeltaSeconds :type Float%20%28single-precision%29)))

(event EventDealDamage
  (params (Damage :type Float%20%28single-precision%29%20%28by%20ref%29))
  (bind _output_get (Variables|Default|SetHealth (- (Variables|Default|GetHealth) Damage)))
  (if (<= _output_get 0.0)
    (CallFunction|OnHealthZero)))

(event EventOnHealthZero
  (params (Interactor :type Actor%20Object%20Reference))
  (Actor|DestroyActor))

(fn ConstructionScript)

(fn GetHealth
  (return (Variables|Default|GetHealth)))

(fn IsShootable
  (params (Interactor :type Actor%20Object%20Reference))
  (return true))