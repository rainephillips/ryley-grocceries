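; An interactable hazard actor that trips the player and hurls a box at them when they enter its capsule trigger.
; On overlap by a "Player"-tagged RG_PlayerCharacter, it calls TripPlayer and spawns a scaled-up BP_Box at its SpawnPoint.
; The box's cube gets a velocity-change impulse toward the player, scaled by Force, and is destroyed after a short delay.
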(event OnComponentBeginOverlap(Capsule)
  (params (OverlappedComponent :type Primitive%20Component%20Object%20Reference) (OtherActor :type Actor%20Object%20Reference) (OtherComp :type Primitive%20Component%20Object%20Reference) (OtherBodyIndex :type Integer) (bFromSweep :type Boolean) (SweepResult :type Hit%20Result%20Structure%20%28by%20ref%29))
  (bind _spawnpoint (Variables|Default|GetSpawnPoint))
  (bind _returnvalue (Transformation|GetWorldLocation _spawnpoint))
  (if (and (Utilities|IsValid OtherActor) (Actor|ActorHasTag OtherActor "Player"))
    (bind _asrg_player_character (Utilities|Casting|CastToRG_PlayerCharacter OtherActor))
    (Class|RGPlayerCharacter|TripPlayer _asrg_player_character)
    (bind _returnvalue_2 (Game|SpawnActorfromClass "/Game/Blueprints/Actors/Gameplay/BP_Box.BP_Box_C" (Math|Transform|MakeTransform _returnvalue "0, 0, 0" "4.000000,4.000000,4.000000") "Undefined" "MultiplyWithRoot" 0 0))
    (Physics|AddImpulse (Variables|/Game/Blueprints/Actors/Gameplay/BP_Box.BP_Box_C|GetCube _returnvalue_2) (* (Math|Vector|Normalize (- (Transformation|GetActorLocation _asrg_player_character) _returnvalue)) (Variables|Default|GetForce)) "None" true)
    (Utilities|FlowControl|Delay 5.0)
    (Actor|DestroyActor _returnvalue_2)))

(event EventBeginPlay)

(event Collision|EventActorBeginOverlap
  (params (OtherActor :type Actor%20Object%20Reference)))

(event EventTick
  (params (DeltaSeconds :type Float%20%28single-precision%29)))

(fn ConstructionScript)