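; BP_Trapdoor is a trapdoor actor that trips the player and swings open when stepped on.
; A physics constraint is bound to the mesh, whose starting transform is cached at BeginPlay.
; When a Player-tagged RG_PlayerCharacter overlaps the box, it calls TripPlayer and frees the constraint's Swing2 limit.
; After the ResetTimer delay, it teleports the mesh back and locks the swing again.
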(event OnComponentBeginOverlap(Box)
  (params (OverlappedComponent :type Primitive%20Component%20Object%20Reference) (OtherActor :type Actor%20Object%20Reference) (OtherComp :type Primitive%20Component%20Object%20Reference) (OtherBodyIndex :type Integer) (bFromSweep :type Boolean) (SweepResult :type Hit%20Result%20Structure%20%28by%20ref%29))
  (if (and (Utilities|IsValid OtherActor) (Actor|ActorHasTag OtherActor "Player"))
    (bind _asrg_player_character (Utilities|Casting|CastToRG_PlayerCharacter OtherActor))
    (Class|RGPlayerCharacter|TripPlayer _asrg_player_character)
    (Class|PhysicsConstraintComponent|SetAngularSwing2Limit (Variables|Default|GetPhysicsConstraint) "ACM_Free" 0.0)
    (Utilities|FlowControl|Delay (Variables|Default|GetResetTimer))
    (Transformation|SetWorldTransform (Variables|Default|GetStaticMesh) (Variables|Default|GetStartTransform) false true)
    (Class|PhysicsConstraintComponent|SetAngularSwing2Limit (Variables|Default|GetPhysicsConstraint) "ACM_Locked" 0.0)))

(event EventBeginPlay
  (Class|PhysicsConstraintComponent|SetConstrainedComponents (Variables|Default|GetPhysicsConstraint) (Variables|Default|GetStaticMesh) "None" 0 "None")
  (Variables|Default|SetStartTransform (Transformation|GetWorldTransform (Variables|Default|GetStaticMesh))))

(event EventTick
  (params (DeltaSeconds :type Float%20%28single-precision%29)))

(fn ConstructionScript)