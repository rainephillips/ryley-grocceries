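; BP_Spring is a launch pad actor that flings the player along its Base's up vector.
; At BeginPlay a physics constraint takes the LaunchPlatform as a constrained component.
; When an actor tagged Player enters the Box, it trips the RG_PlayerCharacter and pushes both character and platform with the same Force.
; An Active flag is set on trigger and cleared after three seconds, but nothing here reads it.
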(event OnComponentBeginOverlap(Box)
  (params (OverlappedComponent :type Primitive%20Component%20Object%20Reference) (OtherActor :type Actor%20Object%20Reference) (OtherComp :type Primitive%20Component%20Object%20Reference) (OtherBodyIndex :type Integer) (bFromSweep :type Boolean) (SweepResult :type Hit%20Result%20Structure%20%28by%20ref%29))
  (bind _base (Variables|Default|GetBase))
  (bind _force (Variables|Default|GetForce))
  (bind _returnvalue (Math|Vector|GetUpVector _base))
  (bind _returnvalue_2 (* _returnvalue _force))
  (if (and (Utilities|IsValid OtherActor) (Actor|ActorHasTag OtherActor "Player"))
    (Variables|Default|SetbActive true)
    (bind _asrg_player_character (Utilities|Casting|CastToRG_PlayerCharacter OtherActor))
    (Class|RGPlayerCharacter|TripPlayer _asrg_player_character)
    (Class|RGPlayerCharacter|AddForce _asrg_player_character _returnvalue_2)
    (Physics|AddForce (Variables|Default|GetLaunchPlatform) _returnvalue_2 "None" true)
    (Utilities|FlowControl|Delay 3.0)
    (Variables|Default|SetbActive false)))

(event EventBeginPlay
  (Class|PhysicsConstraintComponent|SetConstrainedComponents (Variables|Default|GetPhysicsConstraint) (Variables|Default|GetLaunchPlatform) "None" 0 "None"))

(event Collision|EventActorBeginOverlap
  (params (OtherActor :type Actor%20Object%20Reference)))

(fn ConstructionScript)